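; NPC AI controller that drives patrol and target detection for side-scroller characters.
; On BeginPlay it sets up the PatrolData blackboard and runs the EnemyBehaviour behavior tree.
; AI perception writes sensed actors lacking the "Enemy" tag to the enemy key and clears it when sensing fails.
; FindPatrolRoute seeds NextWaypoint with the controlled pawn's first patrol point.
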(event OnTargetPerceptionUpdated(AIPerception)
  (params (Actor :type Actor%20Object%20Reference) (Stimulus :type AI%20Stimulus%20Structure))
  (bind _blackboardcomp (Variables|Default|GetBlackBoardComp))
  (if (not (Actor|ActorHasTag Actor "Enemy"))
    (if (.bsuccessfullysensed Stimulus)
      (AI|Components|Blackboard|SetValueasObject _blackboardcomp (Variables|Default|GetEnemyKey) Actor)
      (else
        (AI|Components|Blackboard|ClearValue _blackboardcomp (Variables|Default|GetEnemyKey))))))

(event EventBeginPlay
  (bind _blackboardcomponent (Class|AIController|UseBlackboard "/Game/NPC/AI/PatrolData.PatrolData"))
  (AI|RunBehaviorTree "/Game/NPC/AI/EnemyBehaviour.EnemyBehaviour")
  (Variables|Default|SetBlackBoardComp _blackboardcomponent))

(fn ConstructionScript)

(fn FindPatrolRoute
  (params (BlackBoard :type Blackboard%20Component%20Object%20Reference))
  (bind _asside_scroller_character (Utilities|Casting|CastToSideScrollerCharacter (Pawn|GetControlledPawn)))
  (AI|Components|Blackboard|SetValueasObject BlackBoard (Utilities|Name|MakeLiteralName "NextWaypoint") (Utilities|Array|Get(acopy) (Variables|/Game/Player/SideScrollerBP/Blueprints/SideScrollerCharacter.SideScrollerCharacter_C|GetPatrolPoints _asside_scroller_character))))
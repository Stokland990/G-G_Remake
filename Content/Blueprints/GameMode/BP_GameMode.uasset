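; BP_GameMode is a game mode Blueprint that runs a minutes-and-seconds countdown to game over.
; Tick feeds a one-second Delay, so the countdown steps about once per second, rolling Seconds over to 59 and decrementing Minutes.
; When both counters equal zero, it prints a red GAME OVER message and pauses the game.
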(event EventTick
  (params (DeltaSeconds :type Float%20%28single-precision%29))
  (Utilities|FlowControl|Delay 1.0)
  (Variables|Default|SetSeconds (- (Variables|Default|GetSeconds) 1))
  (if (< (Variables|Default|GetSeconds) 0)
    (Variables|Default|SetMinutes (- (Variables|Default|GetMinutes) 1))
    (Variables|Default|SetSeconds 59))
  (if (== 0 (Variables|Default|GetSeconds))
    (if (== 0 (Variables|Default|GetMinutes))
      (Development|PrintString "GAME OVER" true true "(R=1.000000,G=0.000000,B=0.000000,A=1.000000)")
      (Game|SetGamePaused true))))

(fn ConstructionScript)
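; BP_DoublePlatform_A is one half of a paired moving platform in a side-scroller, moving between its start position and an EndPoint location.
; When the SideScrollerCharacter overlaps PlayerTouch, it tells its partner PlatformB to reverse and plays its PlatformMove timeline, which lerps the platform toward the end.
; A ReversePlatformA event runs the timeline backward, and playback rate is set from a speed variable on BeginPlay.
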(event OnComponentBeginOverlap(PlayerTouch)
  (params (OverlappedComponent :type Primitive%20Component%20Object%20Reference) (OtherActor :type Actor%20Object%20Reference) (OtherComp :type Primitive%20Component%20Object%20Reference) (OtherBodyIndex :type Integer) (bFromSweep :type Boolean) (SweepResult :type Hit%20Result%20Structure%20%28by%20ref%29))
  (Utilities|Casting|CastToSideScrollerCharacter OtherActor)
  (Default|ReversePlatformB (Variables|Default|GetPlatformB))
  (bind _newtrack_0 (Timeline|PlatformMove Play)
    (:Update
      (Transformation|SetWorldLocation (Variables|Default|GetPlatform) (Math|Vector|Lerp(Vector) (Variables|Default|GetStartLocationA) (Variables|Default|GetEndLocationA) _newtrack_0) false false))))

(event Custom|ReversePlatformA
  (bind _newtrack_0 (Timeline|PlatformMove Reverse)
    (:Update
      (Transformation|SetWorldLocation (Variables|Default|GetPlatform) (Math|Vector|Lerp(Vector) (Variables|Default|GetStartLocationA) (Variables|Default|GetEndLocationA) _newtrack_0) false false))))

(event EventBeginPlay
  (Variables|Default|SetStartLocationA (Transformation|GetWorldLocation (Variables|Default|GetPlatform)))
  (Variables|Default|SetEndLocationA (Transformation|GetWorldLocation (Variables|/Script/Engine.Actor|GetRootComponent (Variables|Platform|GetEndPoint))))
  (Components|Timeline|SetPlayRate (Variables|Default|GetPlatformMove) (Variables|Platform|GetPlarformSpeed)))

(fn ConstructionScript)
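; Door actor that swings open and shut according to the state of a referenced Lever.
; BeginPlay caches the actor's rotation, and Tick polls the Lever's IsLever flag to play a Timeline forward or reverse it.
; The Timeline track supplies a yaw offset, combined with the cached rotation and applied as the Door's world rotation.
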(event EventBeginPlay
  (Variables|Default|SetInitial%20Rotation (Transformation|GetActorRotation)))

(event EventTick
  (params (DeltaSeconds :type Float%20%28single-precision%29))
  (if (Variables|/Game/Blueprints/Actors/Lever.Lever_C|GetisLever (Variables|Lever|GetLever))
    (bind _newtrack_0 (Timeline|Timeline_0 Play)
      (:Update
        (Transformation|SetWorldRotation (Variables|Default|GetDoor) (Math|Rotator|CombineRotators (Variables|Default|GetInitial%20Rotation) (Math|Rotator|MakeRotator 0.0 0.0 _newtrack_0)) false false)))
    (else
      (Timeline|Timeline_0 Reverse))))

(fn ConstructionScript)
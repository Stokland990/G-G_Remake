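; DoublePlatform_B is one half of a linked pair of moving platforms, working with a referenced PlatformA.
; At BeginPlay it stores its own location as the start and the same X/Y at PlatformA's height as the end.
; A timeline lerps it between them: ReversePlatformB plays it toward the end, while SideScrollerCharacter overlap with PlayerTouch reverses it toward the start and calls ReversePlatformA on the partner.
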(event OnComponentBeginOverlap(PlayerTouch)
  (params (OverlappedComponent :type Primitive%20Component%20Object%20Reference) (OtherActor :type Actor%20Object%20Reference) (OtherComp :type Primitive%20Component%20Object%20Reference) (OtherBodyIndex :type Integer) (bFromSweep :type Boolean) (SweepResult :type Hit%20Result%20Structure%20%28by%20ref%29))
  (Utilities|Casting|CastToSideScrollerCharacter OtherActor)
  (Default|ReversePlatformA (Variables|Default|GetPlatformA))
  (bind _newtrack_0 (Timeline|Timeline_0 Reverse)
    (:Update
      (Transformation|SetWorldLocation (Variables|Default|GetPlatform) (Math|Vector|Lerp(Vector) (Variables|Default|GetStartLocationB) (Variables|Default|GetEndLocationB) _newtrack_0) false false))))

(event Custom|ReversePlatformB
  (bind _newtrack_0 (Timeline|Timeline_0 Play)
    (:Update
      (Transformation|SetWorldLocation (Variables|Default|GetPlatform) (Math|Vector|Lerp(Vector) (Variables|Default|GetStartLocationB) (Variables|Default|GetEndLocationB) _newtrack_0) false false))))

(event EventBeginPlay
  (Variables|Default|SetStartLocationB (Transformation|GetWorldLocation (Variables|Default|GetPlatform)))
  (Variables|Default|SetEndLocationB (Math|Vector|MakeVector (.x (Variables|Default|GetStartLocationB)) (.y (Variables|Default|GetStartLocationB)) (.z (Transformation|GetWorldLocation (Variables|/Game/Blueprints/Actors/DoublePlatform_A.DoublePlatform_A_C|GetPlatform (Variables|Default|GetPlatformA)))))))

(fn ConstructionScript)
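; Lever actor for a side-scroller that the player toggles to drive a linked Door.
; OnLeverUse alternates through a FlipFlop, setting IsLever and playing or reversing a timeline that rolls LeverArm relative to the actor's starting rotation.
; Every timeline update calls DoorOpen on the Door, in both directions.
; A Box overlap sets IsNearLever on the SideScrollerCharacter while it is in range.
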(event OnComponentBeginOverlap(Box)
  (params (OverlappedComponent :type Primitive%20Component%20Object%20Reference) (OtherActor :type Actor%20Object%20Reference) (OtherComp :type Primitive%20Component%20Object%20Reference) (OtherBodyIndex :type Integer) (bFromSweep :type Boolean) (SweepResult :type Hit%20Result%20Structure%20%28by%20ref%29))
  (bind _asside_scroller_character (Utilities|Casting|CastToSideScrollerCharacter OtherActor))
  (Variables|/Game/Player/SideScrollerBP/Blueprints/SideScrollerCharacter.SideScrollerCharacter_C|SetIsNearLever _asside_scroller_character true))

(event OnComponentEndOverlap(Box)
  (params (OverlappedComponent :type Primitive%20Component%20Object%20Reference) (OtherActor :type Actor%20Object%20Reference) (OtherComp :type Primitive%20Component%20Object%20Reference) (OtherBodyIndex :type Integer))
  (bind _asside_scroller_character (Utilities|Casting|CastToSideScrollerCharacter OtherActor))
  (Variables|/Game/Player/SideScrollerBP/Blueprints/SideScrollerCharacter.SideScrollerCharacter_C|SetIsNearLever _asside_scroller_character false))

(event Custom|OnLeverUse
  ;[1 1 1] Mechanics of lever use
  (Utilities|FlowControl|FlipFlop
    (:A
      (Variables|Default|SetisLever true)
      (bind _newtrack_0 (Timeline|Timeline_0 Play)
        (:Update
          (Transformation|SetWorldRotation (Variables|Default|GetLeverArm) (Math|Rotator|CombineRotators (Variables|Default|GetInitial%20Rotation) (Math|Rotator|MakeRotator _newtrack_0 0.0 0.0)) false false)
          (Default|DoorOpen (Variables|Door|GetDoor)))))
    (:B
      (Variables|Default|SetisLever false)
      (Timeline|Timeline_0 Reverse))))

(event EventBeginPlay
  ;[1 1 1] GetCurrentRotation
  (Variables|Default|SetInitial%20Rotation (Transformation|GetActorRotation)))

(fn ConstructionScript)